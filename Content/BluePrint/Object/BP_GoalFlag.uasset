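; BP_GoalFlag is the level-end goal flag that scores the player on touch and begins loading the win level.
; On box overlap it hands the player its goal height and landing positions and marks it finished.
; Once only, height thresholds pick a point tier, reveal that score sprite and send the points to the game instance.
; Timelines then lower the flag and raise the score, before collision is disabled and 999WIN streams in hidden.
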(event `self.ReceiveBeginPlay`
  (`SceneComponent.SetVisibility` (`self.100`) false true)
  (`SceneComponent.SetVisibility` (`self.200`) false true)
  (`SceneComponent.SetVisibility` (`self.400`) false true)
  (`SceneComponent.SetVisibility` (`self.800`) false true)
  (`SceneComponent.SetVisibility` (`self.2000`) false true)
  (`SceneComponent.SetVisibility` (`self.5000`) false true))

(event `self.Box.OnComponentBeginOverlap`
  (params (OverlappedComponent :type "PrimitiveComponent Object Reference") (OtherActor :type "Actor Object Reference") (OtherComp :type "PrimitiveComponent Object Reference") (OtherBodyIndex :type Integer) (bFromSweep :type Boolean) (SweepResult :type "HitResult Structure (by ref)"))
  (bind _asbp_player (cast `/Game/BluePrint/BP_Player` OtherActor))
  (bind _output_get (set `/Game/BluePrint/BP_Player.GoalHeight` (`self.K2_GetActorLocation` _asbp_player) _asbp_player))
  (set `/Game/BluePrint/BP_Player.GoalDown_Pos` (`SceneComponent.K2_GetComponentLocation` (`self.Player_Goal_Pos_Down`)) _asbp_player)
  (set `/Game/BluePrint/BP_Player.GoalDownRight_Pos` (`SceneComponent.K2_GetComponentLocation` (`self.Player_Goal_Pos_Down_Right`)) _asbp_player)
  (set `/Game/BluePrint/BP_Player.bGoal` true _asbp_player)
  (set `/Game/BluePrint/BP_Player.bFinish` true _asbp_player)
  (`/Engine/EditorBlueprintResources/StandardMacros.DoOnce` false
    (:`Completed`
      (bind _z (.z _output_get))
      (if (>= _z 50.0)
        (if (>= _z 80.0)
          (if (>= _z 110.0)
            (if (>= _z 140.0)
              (if (>= _z 165.0)
                (set `self.GoalPoint` 5000)
                (`SceneComponent.SetVisibility` (`self.5000`) true true)
                (else
                  (set `self.GoalPoint` 2000)
                  (`SceneComponent.SetVisibility` (`self.2000`) true true)))
              (else
                (set `self.GoalPoint` 800)
                (`SceneComponent.SetVisibility` (`self.800`) true true)))
            (else
              (set `self.GoalPoint` 400)
              (`SceneComponent.SetVisibility` (`self.400`) true true)))
          (else
            (set `self.GoalPoint` 200)
            (`SceneComponent.SetVisibility` (`self.200`) true true)))
        (else
          (set `self.GoalPoint` 100)
          (`SceneComponent.SetVisibility` (`self.100`) true true)))
      (`/Game/BluePrint/BP_GameInstance.Get_Point` (cast `/Game/BluePrint/BP_GameInstance` (`GameplayStatics.GetGameInstance`) :!pure true) (`self.GoalPoint`))
      (`GameplayStatics.PlaySound2D` "/Game/Sound/SE/SE_Goal.SE_Goal" 1.0 1.0 0.0 null null)
      (bind (_direction _alpha) (`Timeline|Timeline_GoalFlag`)
        (:`Update`
          (`SceneComponent.K2_SetRelativeLocation` (`self.PaperSprite3`) (`KismetMathLibrary.VLerp` (-8.0 1.0 143.0) (-8.0 1.0 20.0) _alpha) false false)
          (bind (_direction_2 _alpha_2) (`Timeline|TimeLine_FlagPoint`)
            (:`Update`
              (`SceneComponent.K2_SetRelativeLocation` (`self.FlagPoint`) (`KismetMathLibrary.VLerp` (6.0 1.0 30.0) (6.0 1.0 145.0) _alpha_2) false false))))
        (:`Finished`
          (`KismetSystemLibrary.Delay` 0.5)
          (`PrimitiveComponent.SetCollisionEnabled` (`self.Box`) "NoCollision")
          (`GameplayStatics.LoadStreamLevel` "999WIN"))))))

(fn `UserConstructionScript`)