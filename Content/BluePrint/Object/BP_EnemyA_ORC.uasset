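; Paper2D orc enemy that patrols slowly, turning around at BeginPlay and whenever a hit leaves its X velocity at zero.
; Side-box overlap damages the player, or the orc if the player is melee attacking, which swaps it for an impulse-launched corpse.
; Top-box stomps bounce the player and play a death flipbook; both kills award points with sound and popup text.
; Tick's shell-state logic sits behind constant-false branches and never runs.
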(event `self.ReceiveTick`
  (params (DeltaSeconds :type "Float (single-precision)"))
  (bind _sprite (`self.Sprite`))
  ;[1 1 1] Tick_Walk
  (if false
    (if false
      (set `CharacterMovementComponent.MaxWalkSpeed` 200.0 (`self.CharacterMovement`))
      (`self.AddMovementInput` (`self.GetActorForwardVector`))
      (else
        (`/Engine/EditorBlueprintResources/StandardMacros.DoOnce` false :!label _label
          (:`Completed`
            (`KismetSystemLibrary.Delay` 5.0)
            (if false
              (goto _label :!via `Reset`)
              (else
                (`PaperFlipbookComponent.SetFlipbook` _sprite "/Game/Art/Sprite/31_Enemy_return.31_Enemy_return")
                (`KismetSystemLibrary.Delay` (`PaperFlipbookComponent.GetFlipbookLength` _sprite))
                (if false
                  (`PaperFlipbookComponent.SetFlipbook` (`self.Sprite`) "/Game/Art/Sprite/31_Enemy_shell.31_Enemy_shell")
                  (goto _label :!via `Reset`))))))))
    (else
      (set `CharacterMovementComponent.MaxWalkSpeed` 20.0 (`self.CharacterMovement`))
      (`self.AddMovementInput` (`self.GetActorForwardVector`)))))

(event `self.ReceiveBeginPlay`
  ;[1 1 1] Begin_Rotation
  (`self.K2_SetActorRotation` (`KismetMathLibrary.ComposeRotators` (struct :`Yaw` 180.0) (`self.K2_GetActorRotation`))))

(event `self.ReceiveHit`
  (params (MyComp :type "PrimitiveComponent Object Reference") (Other :type "Actor Object Reference") (OtherComp :type "PrimitiveComponent Object Reference") (bSelfMoved :type Boolean) (HitLocation :type "Vector Structure") (HitNormal :type "Vector Structure") (NormalImpulse :type "Vector Structure") (Hit :type "HitResult Structure (by ref)"))
  (bind _returnvalue_x (`KismetMathLibrary.BreakVector` (`self.GetVelocity`)))
  ;[1 1 1] Attack&Reverse
  (if (== 0.0 _returnvalue_x)
    (`/Engine/EditorBlueprintResources/StandardMacros.DoOnce` false :!label _label_2
      (:`Completed`
        (`self.K2_SetActorRotation` (`KismetMathLibrary.ComposeRotators` (struct :`Yaw` 180.0) (`self.K2_GetActorRotation`)))
        (`KismetSystemLibrary.Delay` 0.2)
        (goto _label_2 :!via `Reset`)))))

(event `self.Box_Attack.OnComponentBeginOverlap`
  (params (OverlappedComponent :type "PrimitiveComponent Object Reference") (OtherActor :type "Actor Object Reference") (OtherComp :type "PrimitiveComponent Object Reference") (OtherBodyIndex :type Integer) (bFromSweep :type Boolean) (SweepResult :type "HitResult Structure (by ref)"))
  ;[1 1 1] Attack&Reverse
  (bind _asbp_player (cast `/Game/BluePrint/BP_Player` OtherActor))
  (if (`/Game/BluePrint/BP_Player.bMelee_Attack` _asbp_player)
    (`GameplayStatics.ApplyDamage` self 1.0)
    (else
      (`GameplayStatics.ApplyDamage` _asbp_player 1.0))))

(event `self.Box_Top.OnComponentBeginOverlap`
  (params (OverlappedComponent :type "PrimitiveComponent Object Reference") (OtherActor :type "Actor Object Reference") (OtherComp :type "PrimitiveComponent Object Reference") (OtherBodyIndex :type Integer) (bFromSweep :type Boolean) (SweepResult :type "HitResult Structure (by ref)"))
  ;[1 1 1] Press_Death
  (bind _asbp_player (cast `/Game/BluePrint/BP_Player` OtherActor))
  (`/Engine/EditorBlueprintResources/StandardMacros.DoOnce` false
    (:`Completed`
      (`self.LaunchCharacter` _asbp_player (0.0 0.0 200.0) false true)
      (`/Game/BluePrint/BP_GameInstance.Get_Point` (cast `/Game/BluePrint/BP_GameInstance` (`GameplayStatics.GetGameInstance`) :!pure true) 100)
      (`PaperFlipbookComponent.SetFlipbook` (`self.Sprite`) "/Game/Art/Sprite/orc_5/Orc-Death1.Orc-Death1")
      (`GameplayStatics.PlaySound2D` "/Game/Sound/SE/SE_Stomp.SE_Stomp" 1.0 1.0 0.0 null null)
      (`|SpawnActorFromClass` "/Game/BluePrint/Object/Spawn/BP_Text_100.BP_Text_100_C" (`KismetMathLibrary.MakeTransform` (+ (0.0 0.0 16.0) (`self.K2_GetActorLocation`))) "Undefined" "OverrideRootScale" null null)
      (`CharacterMovementComponent.DisableMovement` (`self.CharacterMovement`))
      (`self.SetActorEnableCollision` false)
      (`self.SetLifeSpan` 1.0))))

(event `self.ReceiveAnyDamage`
  (params (Damage :type "Float (single-precision)") (DamageType :type "DamageType Object Reference") (InstigatedBy :type "Controller Object Reference") (DamageCauser :type "Actor Object Reference"))
  ;[1 1 1] Hit_Death
  (`self.K2_DestroyActor`)
  (`/Game/BluePrint/BP_GameInstance.Get_Point` (cast `/Game/BluePrint/BP_GameInstance` (`GameplayStatics.GetGameInstance`) :!pure true) 100)
  (`GameplayStatics.PlaySound2D` "/Game/Sound/SE/SE_Kick.SE_Kick" 1.0 1.0 0.0 null null)
  (bind _returnvalue (`|SpawnActorFromClass` "/Game/BluePrint/Object/Spawn/BP_EnemmyA_Death.BP_EnemmyA_Death_C" (`self.GetTransform`) "Undefined" "OverrideRootScale" null null))
  (`PrimitiveComponent.AddImpulse` (`/Game/BluePrint/Object/Spawn/BP_EnemmyA_Death.PaperSprite` _returnvalue) (0.0 0.0 256.0) "None" false)
  (`|SpawnActorFromClass` "/Game/BluePrint/Object/Spawn/BP_Text_100.BP_Text_100_C" (`KismetMathLibrary.MakeTransform` (+ (0.0 0.0 16.0) (`self.K2_GetActorLocation`))) "Undefined" "OverrideRootScale" null null))

(fn `UserConstructionScript`)