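; BP_Arrow is an arrow actor that damages BP_Player on contact.
; On overlap it applies damage to the player, or to itself if the player is in a melee attack.
; On hit, a nonzero X normal plays a block-stop sound, otherwise a player takes damage, and the arrow is destroyed either way.
; Cast-chain macros Enemmy and NoDamage filter enemy and block types but are unused by the event graph.
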(event `self.ReceiveActorBeginOverlap`
  (params (OtherActor :type "Actor Object Reference"))
  (bind _asbp_player (cast `/Game/BluePrint/BP_Player` OtherActor))
  (if (`/Game/BluePrint/BP_Player.bMelee_Attack` _asbp_player)
    (`GameplayStatics.ApplyDamage` self 1.0)
    (else
      (`GameplayStatics.ApplyDamage` _asbp_player 1.0))))

(event `self.ReceiveHit`
  (params (MyComp :type "PrimitiveComponent Object Reference") (Other :type "Actor Object Reference") (OtherComp :type "PrimitiveComponent Object Reference") (bSelfMoved :type Boolean) (HitLocation :type "Vector Structure") (HitNormal :type "Vector Structure") (NormalImpulse :type "Vector Structure") (Hit :type "HitResult Structure (by ref)"))
  (if (!= 0.0 (.x HitNormal))
    (`GameplayStatics.PlaySound2D` "/Game/Sound/SE/SE_Block_stop.SE_Block_stop" 1.0 1.0 0.0 null null)
    (else
      (bind _asbp_player (cast `/Game/BluePrint/BP_Player` Other)
        (:`then`
          (`GameplayStatics.ApplyDamage` _asbp_player 1.0))
        (:`CastFailed`
          _))))
  (`self.K2_DestroyActor`))

(fn `UserConstructionScript`)