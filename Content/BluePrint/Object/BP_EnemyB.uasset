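; Koopa-style shelled enemy that patrols, turns at walls and damages the player on side contact.
; Shell and Kick flags drive its state: stomps on top boxes toggle shell, slide or stop, side touches kick it, and an idle shell revives after a delay.
; A sliding shell damages players and enemies, and rebounds off other objects while damaging blocks.
; Stomps and death award 200 points; any damage swaps it for a launched death actor.
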(event `self.ReceiveBeginPlay`
  ;[1 1 1] Begin_Rotation
  (`self.K2_SetActorRotation` (`KismetMathLibrary.ComposeRotators` (struct :`Yaw` 180.0) (`self.K2_GetActorRotation`))))

(event `self.ReceiveTick`
  (params (DeltaSeconds :type "Float (single-precision)"))
  (bind _sprite (`self.Sprite`))
  ;[1 1 1] Tick_Walk
  (if (`self.bShell`)
    (if (`self.bKick`)
      (set `CharacterMovementComponent.MaxWalkSpeed` 200.0 (`self.CharacterMovement`))
      (`self.AddMovementInput` (`self.GetActorForwardVector`))
      (else
        (`/Engine/EditorBlueprintResources/StandardMacros.DoOnce` false :!label _label
          (:`Completed`
            (`KismetSystemLibrary.Delay` 5.0)
            (if (`self.bKick`)
              (goto _label :!via `Reset`)
              (else
                (`PaperFlipbookComponent.SetFlipbook` _sprite "/Game/Art/Sprite/31_Enemy_return.31_Enemy_return")
                (`KismetSystemLibrary.Delay` (`PaperFlipbookComponent.GetFlipbookLength` _sprite))
                (if (`self.bKick`)
                  (`PaperFlipbookComponent.SetFlipbook` (`self.Sprite`) "/Game/Art/Sprite/31_Enemy_shell.31_Enemy_shell")
                  (goto _label :!via `Reset`)
                  (else
                    (set `self.bShell` false)
                    (`PaperFlipbookComponent.SetFlipbook` (`self.Sprite`) "/Game/Art/Sprite/30_Enemy_walk.30_Enemy_walk")
                    (goto _label :!via `Reset`)))))))))
    (else
      (set `CharacterMovementComponent.MaxWalkSpeed` 20.0 (`self.CharacterMovement`))
      (`self.AddMovementInput` (`self.GetActorForwardVector`)))))

(event `self.ReceiveHit`
  (params (MyComp :type "PrimitiveComponent Object Reference") (Other :type "Actor Object Reference") (OtherComp :type "PrimitiveComponent Object Reference") (bSelfMoved :type Boolean) (HitLocation :type "Vector Structure") (HitNormal :type "Vector Structure") (NormalImpulse :type "Vector Structure") (Hit :type "HitResult Structure (by ref)"))
  (bind _returnvalue_x (`KismetMathLibrary.BreakVector` (`self.GetVelocity`)))
  ;[1 1 1] Attack&Reverse
  (if (== 0.0 _returnvalue_x)
    (`/Engine/EditorBlueprintResources/StandardMacros.DoOnce` false :!label _label_2
      (:`Completed`
        (`self.Reverse`)
        (`KismetSystemLibrary.Delay` 0.2)
        (goto _label_2 :!via `Reset`)))))

(event `self.Box_Forward.OnComponentBeginOverlap`
  (params (OverlappedComponent :type "PrimitiveComponent Object Reference") (OtherActor :type "Actor Object Reference") (OtherComp :type "PrimitiveComponent Object Reference") (OtherBodyIndex :type Integer) (bFromSweep :type Boolean) (SweepResult :type "HitResult Structure (by ref)"))
  (bind _returnvalue_x (`KismetMathLibrary.BreakVector` (`SceneComponent.GetForwardVector` (`self.CapsuleComponent`))))
  ;[1 1 1] Attack&Reverse
  (if (`self.bKick`)
    (`self.BulletDamage` OtherActor)
    (elif (`self.bShell`)
      (cast `/Game/BluePrint/BP_Player` OtherActor)
      (`self.SoundEffect`
        (:`KickOut`
          (`self.LaunchCharacter` (`KismetMathLibrary.MakeVector` (* -300.0 _returnvalue_x)) true)
          (`self.Reverse`)
          (`PrimitiveComponent.SetCollisionEnabled` (`self.Box_Forward`) "NoCollision" :!label _label_3)
          (`PrimitiveComponent.SetCollisionEnabled` (`self.Box_Back`) "NoCollision")
          (set `self.bKick` true)
          (`KismetSystemLibrary.Delay` 0.2)
          (`PrimitiveComponent.SetCollisionEnabled` (`self.Box_Forward`) "QueryOnly")
          (`PrimitiveComponent.SetCollisionEnabled` (`self.Box_Back`) "QueryOnly")))
      (else
        (bind _asbp_player (cast `/Game/BluePrint/BP_Player` OtherActor))
        (`GameplayStatics.ApplyDamage` _asbp_player 1.0)))))

(event `self.Box_Back.OnComponentBeginOverlap`
  (params (OverlappedComponent :type "PrimitiveComponent Object Reference") (OtherActor :type "Actor Object Reference") (OtherComp :type "PrimitiveComponent Object Reference") (OtherBodyIndex :type Integer) (bFromSweep :type Boolean) (SweepResult :type "HitResult Structure (by ref)"))
  (bind _returnvalue_x (`KismetMathLibrary.BreakVector` (`SceneComponent.GetForwardVector` (`self.CapsuleComponent`))))
  ;[1 1 1] Attack&Reverse
  (if (`self.bKick`)
    (`self.BulletDamage` OtherActor)
    (elif (`self.bShell`)
      (cast `/Game/BluePrint/BP_Player` OtherActor)
      (`self.SoundEffect`
        (:`KickOut`
          (`self.LaunchCharacter` (`KismetMathLibrary.MakeVector` (* 300.0 _returnvalue_x)) true)
          (goto _label_3)))
      (else
        (bind _asbp_player (cast `/Game/BluePrint/BP_Player` OtherActor))
        (`GameplayStatics.ApplyDamage` _asbp_player 1.0)))))

(event `self.Box_Top_Forward.OnComponentBeginOverlap`
  (params (OverlappedComponent :type "PrimitiveComponent Object Reference") (OtherActor :type "Actor Object Reference") (OtherComp :type "PrimitiveComponent Object Reference") (OtherBodyIndex :type Integer) (bFromSweep :type Boolean) (SweepResult :type "HitResult Structure (by ref)"))
  ;[1 1 1] Press_Shell
  (bind _asbp_player (cast `/Game/BluePrint/BP_Player` OtherActor))
  (`self.LaunchCharacter` _asbp_player (0.0 0.0 200.0) false true)
  (`PrimitiveComponent.SetCollisionEnabled` (`self.Box_Top_Forward`) "NoCollision")
  (`PrimitiveComponent.SetCollisionEnabled` (`self.Box_Top_Back`) "NoCollision")
  (if (`self.bKick`)
    (set `self.bKick` false)
    (elif (`self.bShell`)
      (set `self.bKick` true)
      (`self.Reverse`)
      (else
        (set `self.bShell` true))))
  (`PaperFlipbookComponent.SetFlipbook` (`self.Sprite`) "/Game/Art/Sprite/31_Enemy_shell.31_Enemy_shell" :!label _label_4)
  (`self.GetPoint200`)
  (`self.SoundEffect` :!via `Stomp`
    (:`StompOut`
      (`KismetSystemLibrary.Delay` 0.1)
      (`PrimitiveComponent.SetCollisionEnabled` (`self.Box_Top_Forward`) "QueryOnly")
      (`PrimitiveComponent.SetCollisionEnabled` (`self.Box_Top_Back`) "QueryOnly"))))

(event `self.Box_Top_Back.OnComponentBeginOverlap`
  (params (OverlappedComponent :type "PrimitiveComponent Object Reference") (OtherActor :type "Actor Object Reference") (OtherComp :type "PrimitiveComponent Object Reference") (OtherBodyIndex :type Integer) (bFromSweep :type Boolean) (SweepResult :type "HitResult Structure (by ref)"))
  ;[1 1 1] Press_Shell
  (bind _asbp_player (cast `/Game/BluePrint/BP_Player` OtherActor))
  (`self.LaunchCharacter` _asbp_player (0.0 0.0 200.0) false true)
  (`PrimitiveComponent.SetCollisionEnabled` (`self.Box_Top_Forward`) "NoCollision")
  (`PrimitiveComponent.SetCollisionEnabled` (`self.Box_Top_Back`) "NoCollision")
  (if (`self.bKick`)
    (set `self.bKick` false)
    (goto _label_4)
    (elif (`self.bShell`)
      (set `self.bKick` true)
      (goto _label_4)
      (else
        (set `self.bShell` true)
        (goto _label_4)))))

(event `self.ReceiveAnyDamage`
  (params (Damage :type "Float (single-precision)") (DamageType :type "DamageType Object Reference") (InstigatedBy :type "Controller Object Reference") (DamageCauser :type "Actor Object Reference"))
  ;[1 1 1] Hit_Death
  (`self.K2_DestroyActor`)
  (bind _returnvalue (`|SpawnActorFromClass` "/Game/BluePrint/Object/Spawn/BP_EnemmyB_Death.BP_EnemmyB_Death_C" (`self.GetTransform`) "Undefined" "OverrideRootScale" null null))
  (`PrimitiveComponent.AddImpulse` (`/Game/BluePrint/Object/Spawn/BP_EnemmyB_Death.PaperSprite` _returnvalue) (0.0 0.0 256.0) "None" false)
  (`self.GetPoint200`)
  (`self.SoundEffect`))

(fn `Reverse`
  (`self.K2_SetActorRotation` (`KismetMathLibrary.ComposeRotators` (struct :`Yaw` 180.0) (`self.K2_GetActorRotation`))))

(fn `UserConstructionScript`)