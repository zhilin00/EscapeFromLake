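; BP_EnemyA_motor1 is an enemy that creeps along its forward vector each tick, after a 180-degree rotation at BeginPlay.
; Hitting a BP_Block_fix destroys it.
; When Box_Attack overlaps BP_Player, the enemy damages itself if the player's MeleeAttack flag is set, otherwise it damages the player.
; No response to received damage is defined in this graph.
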(event `self.ReceiveBeginPlay`
  ;[1 1 1] Begin_Rotation
  (`self.K2_SetActorRotation` (`KismetMathLibrary.ComposeRotators` (struct :`Yaw` 180.0) (`self.K2_GetActorRotation`))))

(event `self.ReceiveTick`
  (params (DeltaSeconds :type "Float (single-precision)"))
  ;[1 1 1] Tick_Walk
  (`self.AddMovementInput` (`self.GetActorForwardVector`) 0.001))

(event `self.ReceiveHit`
  (params (MyComp :type "PrimitiveComponent Object Reference") (Other :type "Actor Object Reference") (OtherComp :type "PrimitiveComponent Object Reference") (bSelfMoved :type Boolean) (HitLocation :type "Vector Structure") (HitNormal :type "Vector Structure") (NormalImpulse :type "Vector Structure") (Hit :type "HitResult Structure (by ref)"))
  ;[1 1 1] Attack&Reverse
  (cast `/Game/BluePrint/Object/Spawn/BP_Block_fix` Other)
  (`self.K2_DestroyActor`))

(event `self.Box_Attack.OnComponentBeginOverlap`
  (params (OverlappedComponent :type "PrimitiveComponent Object Reference") (OtherActor :type "Actor Object Reference") (OtherComp :type "PrimitiveComponent Object Reference") (OtherBodyIndex :type Integer) (bFromSweep :type Boolean) (SweepResult :type "HitResult Structure (by ref)"))
  ;[1 1 1] Attack&Reverse
  (bind _asbp_player (cast `/Game/BluePrint/BP_Player` OtherActor))
  (if (`/Game/BluePrint/BP_Player.bMelee_Attack` _asbp_player)
    (`GameplayStatics.ApplyDamage` self 1.0)
    (else
      (`GameplayStatics.ApplyDamage` _asbp_player 1.0))))

(fn `UserConstructionScript`)