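; BP_Explosion is a short-lived explosion object that damages the player and expires two seconds after BeginPlay.
; Its Hit event casts the other object to BP_Player and applies damage only when that cast succeeds.
; Two cast-based filter graphs, Enemmy for enemy types and NoDamage for excluding block types, are defined but not called from the event graph.
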(event `self.ReceiveBeginPlay`
  (`self.SetLifeSpan` 2.0))

(event `self.ReceiveHit`
  (params (MyComp :type "PrimitiveComponent Object Reference") (Other :type "Actor Object Reference") (OtherComp :type "PrimitiveComponent Object Reference") (bSelfMoved :type Boolean) (HitLocation :type "Vector Structure") (HitNormal :type "Vector Structure") (NormalImpulse :type "Vector Structure") (Hit :type "HitResult Structure (by ref)"))
  (bind _asbp_player (cast `/Game/BluePrint/BP_Player` Other))
  (`GameplayStatics.ApplyDamage` _asbp_player 1.0))

(fn `UserConstructionScript`)