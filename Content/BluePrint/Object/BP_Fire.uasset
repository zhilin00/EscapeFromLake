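; BP_Fire is a short-lived fire hazard actor that damages the player on overlap.
; Overlapping a BP_Player applies damage, while a Delay driven from Tick destroys the actor after a couple of seconds.
; Helper graphs Enemmy and NoDamage use cast chains to filter for the two enemy types and for non-block objects, but the event graph uses neither.
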(event `self.ReceiveTick`
  (params (DeltaSeconds :type "Float (single-precision)"))
  (`KismetSystemLibrary.Delay` 2.0)
  (`self.K2_DestroyActor`))

(event `self.ReceiveActorBeginOverlap`
  (params (OtherActor :type "Actor Object Reference"))
  (bind _asbp_player (cast `/Game/BluePrint/BP_Player` OtherActor))
  (`GameplayStatics.ApplyDamage` _asbp_player 1.0))

(fn `UserConstructionScript`)