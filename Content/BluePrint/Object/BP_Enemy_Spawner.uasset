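; Enemy spawner actor that, when overlapped, spawns EnemyA, EnemyB or a boss as selected by Type.
; Quantities one to seven spawn a cascading batch at numbered box components, then destroy the spawner.
; Quantity zero enables Tick-driven spawning every five seconds until Box_End overlap destroys it, though the boss loop is unwired.
; The construction script previews the setup through box visibility and enemy sprite.
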(event `self.ReceiveTick`
  (params (DeltaSeconds :type "Float (single-precision)"))
  (if (`self.infinity`)
    (switch `int` (`self.Type`)
      (:`0`
        (`/Engine/EditorBlueprintResources/StandardMacros.DoOnce` false :!label _label
          (:`Completed`
            (bind _returnvalue (`|SpawnActorFromClass` "/Game/BluePrint/Object/BP_EnemyA.BP_EnemyA_C" (`SceneComponent.K2_GetComponentToWorld` (`self.Box1`)) "Undefined" "OverrideRootScale" null null))
            (`Pawn.SpawnDefaultController` _returnvalue)
            (`KismetSystemLibrary.Delay` 5.0)
            (goto _label :!via `Reset`))))
      (:`1`
        (`/Engine/EditorBlueprintResources/StandardMacros.DoOnce` false :!label _label_2
          (:`Completed`
            (bind _returnvalue_2 (`|SpawnActorFromClass` "/Game/BluePrint/Object/BP_EnemyB.BP_EnemyB_C" (`SceneComponent.K2_GetComponentToWorld` (`self.Box1`)) "Undefined" "OverrideRootScale" null null))
            (`Pawn.SpawnDefaultController` _returnvalue_2)
            (`KismetSystemLibrary.Delay` 5.0)
            (goto _label_2 :!via `Reset`))))
      (:`2`
        (`/Engine/EditorBlueprintResources/StandardMacros.DoOnce` false)))))

(event `self.ReceiveActorBeginOverlap`
  (params (OtherActor :type "Actor Object Reference"))
  (switch `int` (`self.Type`)
    (:`0`
      (switch `int` (`self.Quantity`)
        (:`0`
          (set `self.infinity` true))
        (:`1`
          (bind _returnvalue (`|SpawnActorFromClass` "/Game/BluePrint/Object/BP_EnemyA.BP_EnemyA_C" (`SceneComponent.K2_GetComponentToWorld` (`self.Box1`)) "Undefined" "OverrideRootScale" null null :!label _label_3))
          (`Pawn.SpawnDefaultController` _returnvalue)
          (`self.K2_DestroyActor`))
        (:`2`
          (bind _returnvalue_2 (`|SpawnActorFromClass` "/Game/BluePrint/Object/BP_EnemyA.BP_EnemyA_C" (`SceneComponent.K2_GetComponentToWorld` (`self.Box2`)) "Undefined" "OverrideRootScale" null null :!label _label_4))
          (`Pawn.SpawnDefaultController` _returnvalue_2)
          (goto _label_3))
        (:`3`
          (bind _returnvalue_3 (`|SpawnActorFromClass` "/Game/BluePrint/Object/BP_EnemyA.BP_EnemyA_C" (`SceneComponent.K2_GetComponentToWorld` (`self.Box3`)) "Undefined" "OverrideRootScale" null null :!label _label_5))
          (`Pawn.SpawnDefaultController` _returnvalue_3)
          (goto _label_4))
        (:`4`
          (bind _returnvalue_4 (`|SpawnActorFromClass` "/Game/BluePrint/Object/BP_EnemyA.BP_EnemyA_C" (`SceneComponent.K2_GetComponentToWorld` (`self.Box4`)) "Undefined" "OverrideRootScale" null null :!label _label_6))
          (`Pawn.SpawnDefaultController` _returnvalue_4)
          (goto _label_5))
        (:`5`
          (bind _returnvalue_5 (`|SpawnActorFromClass` "/Game/BluePrint/Object/BP_EnemyA.BP_EnemyA_C" (`SceneComponent.K2_GetComponentToWorld` (`self.Box5`)) "Undefined" "OverrideRootScale" null null :!label _label_7))
          (`Pawn.SpawnDefaultController` _returnvalue_5)
          (goto _label_6))
        (:`6`
          (bind _returnvalue_6 (`|SpawnActorFromClass` "/Game/BluePrint/Object/BP_EnemyA.BP_EnemyA_C" (`SceneComponent.K2_GetComponentToWorld` (`self.Box6`)) "Undefined" "OverrideRootScale" null null :!label _label_8))
          (`Pawn.SpawnDefaultController` _returnvalue_6)
          (goto _label_7))
        (:`7`
          (bind _returnvalue_7 (`|SpawnActorFromClass` "/Game/BluePrint/Object/BP_EnemyA.BP_EnemyA_C" (`SceneComponent.K2_GetComponentToWorld` (`self.Box7`)) "Undefined" "OverrideRootScale" null null))
          (`Pawn.SpawnDefaultController` _returnvalue_7)
          (goto _label_8))))
    (:`1`
      (switch `int` (`self.Quantity`)
        (:`0`
          (set `self.infinity` true))
        (:`1`
          (bind _returnvalue_8 (`|SpawnActorFromClass` "/Game/BluePrint/Object/BP_EnemyB.BP_EnemyB_C" (`SceneComponent.K2_GetComponentToWorld` (`self.Box1`)) "Undefined" "OverrideRootScale" null null :!label _label_9))
          (`Pawn.SpawnDefaultController` _returnvalue_8)
          (`self.K2_DestroyActor`))
        (:`2`
          (bind _returnvalue_9 (`|SpawnActorFromClass` "/Game/BluePrint/Object/BP_EnemyB.BP_EnemyB_C" (`SceneComponent.K2_GetComponentToWorld` (`self.Box2`)) "Undefined" "OverrideRootScale" null null :!label _label_10))
          (`Pawn.SpawnDefaultController` _returnvalue_9)
          (goto _label_9))
        (:`3`
          (bind _returnvalue_10 (`|SpawnActorFromClass` "/Game/BluePrint/Object/BP_EnemyB.BP_EnemyB_C" (`SceneComponent.K2_GetComponentToWorld` (`self.Box3`)) "Undefined" "OverrideRootScale" null null :!label _label_11))
          (`Pawn.SpawnDefaultController` _returnvalue_10)
          (goto _label_10))
        (:`4`
          (bind _returnvalue_11 (`|SpawnActorFromClass` "/Game/BluePrint/Object/BP_EnemyB.BP_EnemyB_C" (`SceneComponent.K2_GetComponentToWorld` (`self.Box4`)) "Undefined" "OverrideRootScale" null null :!label _label_12))
          (`Pawn.SpawnDefaultController` _returnvalue_11)
          (goto _label_11))
        (:`5`
          (bind _returnvalue_12 (`|SpawnActorFromClass` "/Game/BluePrint/Object/BP_EnemyB.BP_EnemyB_C" (`SceneComponent.K2_GetComponentToWorld` (`self.Box5`)) "Undefined" "OverrideRootScale" null null :!label _label_13))
          (`Pawn.SpawnDefaultController` _returnvalue_12)
          (goto _label_12))
        (:`6`
          (bind _returnvalue_13 (`|SpawnActorFromClass` "/Game/BluePrint/Object/BP_EnemyB.BP_EnemyB_C" (`SceneComponent.K2_GetComponentToWorld` (`self.Box6`)) "Undefined" "OverrideRootScale" null null :!label _label_14))
          (`Pawn.SpawnDefaultController` _returnvalue_13)
          (goto _label_13))
        (:`7`
          (bind _returnvalue_14 (`|SpawnActorFromClass` "/Game/BluePrint/Object/BP_EnemyB.BP_EnemyB_C" (`SceneComponent.K2_GetComponentToWorld` (`self.Box7`)) "Undefined" "OverrideRootScale" null null))
          (`Pawn.SpawnDefaultController` _returnvalue_14)
          (goto _label_14))))
    (:`2`
      (switch `int` (`self.Quantity`)
        (:`0`
          (set `self.infinity` true))
        (:`1`
          (bind _returnvalue_15 (`|SpawnActorFromClass` "/Game/BluePrint/Object/BP_EnemyBoss.BP_EnemyBoss_C" (`SceneComponent.K2_GetComponentToWorld` (`self.Box1`)) "AlwaysSpawn" "OverrideRootScale" null null))
          (`Pawn.SpawnDefaultController` _returnvalue_15)
          (`self.K2_DestroyActor`))))))

(event `self.Box_End.OnComponentBeginOverlap`
  (params (OverlappedComponent :type "PrimitiveComponent Object Reference") (OtherActor :type "Actor Object Reference") (OtherComp :type "PrimitiveComponent Object Reference") (OtherBodyIndex :type Integer) (bFromSweep :type Boolean) (SweepResult :type "HitResult Structure (by ref)"))
  (set `self.infinity` false)
  (`self.K2_DestroyActor`))

(fn `UserConstructionScript`
  (bind _box_torigger_r (`self.Box_Torigger_R`))
  (`|ExecutionSequence`
    (:`then_0`
      (if (`self.Trigger_R`)
        (`SceneComponent.SetVisibility` _box_torigger_r true false)
        (else
          (`SceneComponent.SetVisibility` _box_torigger_r false false))))
    (:`then_1`
      (switch `int` (`self.Quantity`)
        (:`0`
          (`SceneComponent.SetVisibility` (`self.Box1`) true false :!label _label))
        (:`1`
          (goto _label))
        (:`2`
          (`SceneComponent.SetVisibility` (`self.Box1`) true false)
          (`SceneComponent.SetVisibility` (`self.Box2`) true false))
        (:`3`
          (`SceneComponent.SetVisibility` (`self.Box1`) true false)
          (`SceneComponent.SetVisibility` (`self.Box2`) true false)
          (`SceneComponent.SetVisibility` (`self.Box3`) true false))
        (:`4`
          (`SceneComponent.SetVisibility` (`self.Box1`) true false)
          (`SceneComponent.SetVisibility` (`self.Box2`) true false)
          (`SceneComponent.SetVisibility` (`self.Box3`) true false)
          (`SceneComponent.SetVisibility` (`self.Box4`) true false))
        (:`5`
          (`SceneComponent.SetVisibility` (`self.Box1`) true false)
          (`SceneComponent.SetVisibility` (`self.Box2`) true false)
          (`SceneComponent.SetVisibility` (`self.Box3`) true false)
          (`SceneComponent.SetVisibility` (`self.Box4`) true false)
          (`SceneComponent.SetVisibility` (`self.Box5`) true false))
        (:`6`
          (`SceneComponent.SetVisibility` (`self.Box1`) true false)
          (`SceneComponent.SetVisibility` (`self.Box2`) true false)
          (`SceneComponent.SetVisibility` (`self.Box3`) true false)
          (`SceneComponent.SetVisibility` (`self.Box4`) true false)
          (`SceneComponent.SetVisibility` (`self.Box5`) true false)
          (`SceneComponent.SetVisibility` (`self.Box6`) true false))
        (:`7`
          (`SceneComponent.SetVisibility` (`self.Box1`) true false)
          (`SceneComponent.SetVisibility` (`self.Box2`) true false)
          (`SceneComponent.SetVisibility` (`self.Box3`) true false)
          (`SceneComponent.SetVisibility` (`self.Box4`) true false)
          (`SceneComponent.SetVisibility` (`self.Box5`) true false)
          (`SceneComponent.SetVisibility` (`self.Box6`) true false)
          (`SceneComponent.SetVisibility` (`self.Box7`) true false))))
    (:`then_2`
      (switch `int` (`self.Type`)
        (:`0`
          (`PaperSpriteComponent.SetSprite` (`self.PaperSprite`) "/Game/Art/Sprite/30_Enemy/30_Enemy_0.30_Enemy_0"))
        (:`1`
          (`PaperSpriteComponent.SetSprite` (`self.PaperSprite`) "/Game/Art/Sprite/30_Enemy/31_Enemy_0.31_Enemy_0"))))
    (:`then_3`
      (if (== 0 (`self.Quantity`))
        (`SceneComponent.SetVisibility` (`self.Box_End`) true false)))))