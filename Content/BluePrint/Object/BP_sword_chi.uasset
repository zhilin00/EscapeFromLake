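; BP_sword_chi is a sword object, apparently a projectile, that deals damage in a Mario-style game with blocks and enemies.
; Overlaps apply damage to the other actor.
; Hits play a block-stop sound when the normal has an X component, otherwise apply damage, then destroy the sword either way.
; Enemmy and NoDamage graphs filter enemies and exclude block types by casting, but the event graph never uses them.
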(event `self.ReceiveActorBeginOverlap`
  (params (OtherActor :type "Actor Object Reference"))
  (`GameplayStatics.ApplyDamage` OtherActor 1.0))

(event `self.ReceiveHit`
  (params (MyComp :type "PrimitiveComponent Object Reference") (Other :type "Actor Object Reference") (OtherComp :type "PrimitiveComponent Object Reference") (bSelfMoved :type Boolean) (HitLocation :type "Vector Structure") (HitNormal :type "Vector Structure") (NormalImpulse :type "Vector Structure") (Hit :type "HitResult Structure (by ref)"))
  (if (!= 0.0 (.x HitNormal))
    (`GameplayStatics.PlaySound2D` "/Game/Sound/SE/SE_Block_stop.SE_Block_stop" 1.0 1.0 0.0 null null)
    (else
      (`GameplayStatics.ApplyDamage` Other 1.0)))
  (`self.K2_DestroyActor`))

(fn `UserConstructionScript`)