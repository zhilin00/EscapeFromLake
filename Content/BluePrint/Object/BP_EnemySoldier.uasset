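; BP_EnemySoldier is a flipbook-animated enemy soldier that fights BP_Player with arrows and melee attacks.
; While Shoot is set, Tick launches BP_Arrow characters, paced by a Delay.
; Attack_range overlap clears Shoot and plays one of two random delayed-damage melee attacks; leaving restores shooting.
; Four side boxes deal contact damage, while AnyDamage handles hurt animation and death with points, score popup, sound and timed removal.
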(event `self.ReceiveTick`
  (params (DeltaSeconds :type "Float (single-precision)"))
  (bind _returnvalue_x (`KismetMathLibrary.BreakVector` (`self.GetActorForwardVector`)))
  ;[1 1 1] Tick_Shoot
  (if (`self.bShoot`)
    (`PaperFlipbookComponent.SetFlipbook` (`self.Sprite`) "/Game/Art/Sprite/soldier_boss_3/Soldier-Attack3.Soldier-Attack3")
    (`KismetSystemLibrary.Delay` 1.0)
    (bind _returnvalue (`|SpawnActorFromClass` "/Game/BluePrint/Object/BP_Arrow.BP_Arrow_C" (`SceneComponent.K2_GetComponentToWorld` (`self.Fire_Ball_Pos1`)) "AlwaysSpawn" "OverrideRootScale" null null))
    (`self.SpawnDefaultController` _returnvalue)
    (`self.LaunchCharacter` _returnvalue (`KismetMathLibrary.MakeVector` (* 200.0 _returnvalue_x)) false false)
    (`PaperFlipbookComponent.SetFlipbook` (`self.Sprite`) "/Game/Art/Sprite/soldier_boss_3/Soldier-Idle1.Soldier-Idle1")))

(event `self.Box_Forward.OnComponentBeginOverlap`
  (params (OverlappedComponent :type "PrimitiveComponent Object Reference") (OtherActor :type "Actor Object Reference") (OtherComp :type "PrimitiveComponent Object Reference") (OtherBodyIndex :type Integer) (bFromSweep :type Boolean) (SweepResult :type "HitResult Structure (by ref)"))
  ;[1 1 1] Attack&Reverse
  (bind _asbp_player (cast `/Game/BluePrint/BP_Player` OtherActor))
  (`GameplayStatics.ApplyDamage` _asbp_player 1.0))

(event `self.Box_Back.OnComponentBeginOverlap`
  (params (OverlappedComponent :type "PrimitiveComponent Object Reference") (OtherActor :type "Actor Object Reference") (OtherComp :type "PrimitiveComponent Object Reference") (OtherBodyIndex :type Integer) (bFromSweep :type Boolean) (SweepResult :type "HitResult Structure (by ref)"))
  ;[1 1 1] Attack&Reverse
  (bind _asbp_player (cast `/Game/BluePrint/BP_Player` OtherActor))
  (`GameplayStatics.ApplyDamage` _asbp_player 1.0))

(event `self.Box_Top_Forward.OnComponentBeginOverlap`
  (params (OverlappedComponent :type "PrimitiveComponent Object Reference") (OtherActor :type "Actor Object Reference") (OtherComp :type "PrimitiveComponent Object Reference") (OtherBodyIndex :type Integer) (bFromSweep :type Boolean) (SweepResult :type "HitResult Structure (by ref)"))
  ;[1 1 1] Attack&Reverse
  (bind _asbp_player (cast `/Game/BluePrint/BP_Player` OtherActor))
  (`GameplayStatics.ApplyDamage` _asbp_player 1.0))

(event `self.Box_Top_Back.OnComponentBeginOverlap`
  (params (OverlappedComponent :type "PrimitiveComponent Object Reference") (OtherActor :type "Actor Object Reference") (OtherComp :type "PrimitiveComponent Object Reference") (OtherBodyIndex :type Integer) (bFromSweep :type Boolean) (SweepResult :type "HitResult Structure (by ref)"))
  ;[1 1 1] Attack&Reverse
  (bind _asbp_player (cast `/Game/BluePrint/BP_Player` OtherActor))
  (`GameplayStatics.ApplyDamage` _asbp_player 1.0))

(event `self.attack_range.OnComponentBeginOverlap`
  (params (OverlappedComponent :type "PrimitiveComponent Object Reference") (OtherActor :type "Actor Object Reference") (OtherComp :type "PrimitiveComponent Object Reference") (OtherBodyIndex :type Integer) (bFromSweep :type Boolean) (SweepResult :type "HitResult Structure (by ref)"))
  ;[1 1 1] Attack&Reverse
  (bind _asbp_player (cast `/Game/BluePrint/BP_Player` OtherActor))
  (set `self.bShoot` false)
  (switch `int` (`KismetMathLibrary.RandomInteger` 2)
    (:`0`
      (`PaperFlipbookComponent.SetFlipbook` (`self.Sprite`) "/Game/Art/Sprite/soldier_boss_3/Soldier-Attack1.Soldier-Attack1")
      (`KismetSystemLibrary.Delay` 0.3)
      (if (not (`self.bShoot`))
        (`GameplayStatics.ApplyDamage` _asbp_player 1.0 :!label _label)))
    (:`1`
      (`PaperFlipbookComponent.SetFlipbook` (`self.Sprite`) "/Game/Art/Sprite/soldier_boss_3/Soldier-Attack2.Soldier-Attack2")
      (`KismetSystemLibrary.Delay` 0.4)
      (if (not (`self.bShoot`))
        (goto _label)))))

(event `self.attack_range.OnComponentEndOverlap`
  (params (OverlappedComponent :type "PrimitiveComponent Object Reference") (OtherActor :type "Actor Object Reference") (OtherComp :type "PrimitiveComponent Object Reference") (OtherBodyIndex :type Integer))
  ;[1 1 1] Attack&Reverse
  (cast `/Game/BluePrint/BP_Player` OtherActor)
  (set `self.bShoot` true)
  (`KismetSystemLibrary.Delay` 0.5)
  (`PaperFlipbookComponent.SetFlipbook` (`self.Sprite`) "/Game/Art/Sprite/soldier_boss_3/Soldier-Idle1.Soldier-Idle1"))

(event `self.ReceiveAnyDamage`
  (params (Damage :type "Float (single-precision)") (DamageType :type "DamageType Object Reference") (InstigatedBy :type "Controller Object Reference") (DamageCauser :type "Actor Object Reference"))
  (bind _returnvalue (- (`self.iHealth`) Damage))
  ;[1 1 1] Hit_Death
  (if (== _returnvalue 0.0)
    (`/Game/BluePrint/BP_GameInstance.Get_Point` (cast `/Game/BluePrint/BP_GameInstance` (`GameplayStatics.GetGameInstance`) :!pure true) 1000)
    (`PaperFlipbookComponent.SetFlipbook` (`self.Sprite`) "/Game/Art/Sprite/soldier_boss_3/Soldier-Death1.Soldier-Death1")
    (`GameplayStatics.PlaySound2D` "/Game/Sound/SE/SE_Stomp.SE_Stomp" 1.0 1.0 0.0 null null)
    (`|SpawnActorFromClass` "/Game/BluePrint/Object/Spawn/BP_Text_1000.BP_Text_1000_C" (`KismetMathLibrary.MakeTransform` (+ (0.0 0.0 16.0) (`self.K2_GetActorLocation`))) "Undefined" "OverrideRootScale" null null)
    (`CharacterMovementComponent.DisableMovement` (`self.CharacterMovement`))
    (`self.SetActorEnableCollision` false)
    (`self.SetLifeSpan` 1.0)
    (else
      (set `self.iHealth` _returnvalue)
      (`PaperFlipbookComponent.SetFlipbook` (`self.Sprite`) "/Game/Art/Sprite/soldier_boss_3/Soldier-Hurt1.Soldier-Hurt1")
      (`KismetSystemLibrary.Delay` 0.5)
      (`PaperFlipbookComponent.SetFlipbook` (`self.Sprite`) "/Game/Art/Sprite/soldier_boss_3/Soldier-Idle1.Soldier-Idle1"))))

(fn `Reverse`
  (`self.K2_SetActorRotation` (`KismetMathLibrary.ComposeRotators` (struct :`Yaw` 180.0) (`self.K2_GetActorRotation`))))

(fn `UserConstructionScript`)