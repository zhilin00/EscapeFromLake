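; Breakable 2D brick block that reacts when BP_Player hits it from below, with Style selecting its sprite and debris.
; Mini power-up only bumps it via timelines, while Big, Fire or any damage breaks it once into four impulsed debris pieces before destroying it.
; A hit briefly enables the top trigger, whose Launch macro tosses players and pickups upward, ignores other blocks and damages anything else.
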(event `self.ReceiveBeginPlay`
  (`PrimitiveComponent.SetCollisionEnabled` (`self.Box_Top`) "NoCollision"))

(event `self.Box_Bottom.OnComponentBeginOverlap`
  (params (OverlappedComponent :type "PrimitiveComponent Object Reference") (OtherActor :type "Actor Object Reference") (OtherComp :type "PrimitiveComponent Object Reference") (OtherBodyIndex :type Integer) (bFromSweep :type Boolean) (SweepResult :type "HitResult Structure (by ref)"))
  (cast `/Game/BluePrint/BP_Player` OtherActor)
  (`PrimitiveComponent.SetCollisionEnabled` (`self.Box_Bottom`) "NoCollision")
  (`PrimitiveComponent.SetCollisionEnabled` (`self.Box_Top`) "QueryOnly")
  (switch `/Game/BluePrint/Enum/PowerUp` (`/Game/BluePrint/BP_GameInstance.PowerUp` (cast `/Game/BluePrint/BP_GameInstance` (`GameplayStatics.GetGameInstance`) :!pure true))
    (:`NewEnumerator0`
      ;[1 1 1] BlockUp
      (`self.SoundEffect`
        (:`BlockStopOut`
          (bind (_direction _alpha) (`Timeline|BlockUp` :!via `PlayFromStart`)
            (:`Update`
              (`SceneComponent.K2_SetRelativeLocation` (`self.Box_Collision`) (`KismetMathLibrary.VLerp` (0.0 0.0 0.0) (0.0 0.0 4.0) _alpha) false false))
            (:`Finished`
              (bind (_direction_2 _alpha_2) (`Timeline|BlockDown` :!via `PlayFromStart`)
                (:`Update`
                  (`SceneComponent.K2_SetRelativeLocation` (`self.Box_Collision`) (`KismetMathLibrary.VLerp` (0.0 0.0 4.0) (0.0 0.0 0.0) _alpha_2) false false))
                (:`Finished`
                  (`PrimitiveComponent.SetCollisionEnabled` (`self.Box_Bottom`) "QueryOnly")
                  (`PrimitiveComponent.SetCollisionEnabled` (`self.Box_Top`) "NoCollision"))))))))
    (:`NewEnumerator1`
      (`/Engine/EditorBlueprintResources/StandardMacros.DoOnce` false :!label _label
        (:`Completed`
          (switch `int` (`self.Style`)
            (:`Default`
              ;[1 1 1] BlockBreak
              (`|ExecutionSequence` :!label _label_2
                (:`then_0`
                  (bind _returnvalue (`|SpawnActorFromClass` "/Game/BluePrint/Object/Spawn/BP_Block_Debris0.BP_Block_Debris0_C" (`KismetMathLibrary.MakeTransform` (+ (4.0 0.0 4.0) (`self.K2_GetActorLocation`))) "Undefined" "OverrideRootScale" null null))
                  (`PrimitiveComponent.AddImpulse` (`/Game/BluePrint/Object/Spawn/BP_Block_Debris0.PaperSprite` _returnvalue) (32.0 0.0 128.0) "None" false))
                (:`then_1`
                  (bind _returnvalue_2 (`|SpawnActorFromClass` "/Game/BluePrint/Object/Spawn/BP_Block_Debris0.BP_Block_Debris0_C" (`KismetMathLibrary.MakeTransform` (+ (4.0 0.0 -4.0) (`self.K2_GetActorLocation`))) "Undefined" "OverrideRootScale" null null))
                  (`PrimitiveComponent.AddImpulse` (`/Game/BluePrint/Object/Spawn/BP_Block_Debris0.PaperSprite` _returnvalue_2) (32.0 0.0 64.0) "None" false))
                (:`then_2`
                  (bind _returnvalue_3 (`|SpawnActorFromClass` "/Game/BluePrint/Object/Spawn/BP_Block_Debris0.BP_Block_Debris0_C" (`KismetMathLibrary.MakeTransform` (+ (-4.0 0.0 4.0) (`self.K2_GetActorLocation`))) "Undefined" "OverrideRootScale" null null))
                  (`PrimitiveComponent.AddImpulse` (`/Game/BluePrint/Object/Spawn/BP_Block_Debris0.PaperSprite` _returnvalue_3) (-32.0 0.0 128.0) "None" false))
                (:`then_3`
                  (bind _returnvalue_4 (`|SpawnActorFromClass` "/Game/BluePrint/Object/Spawn/BP_Block_Debris0.BP_Block_Debris0_C" (`KismetMathLibrary.MakeTransform` (+ (-4.0 0.0 -4.0) (`self.K2_GetActorLocation`))) "Undefined" "OverrideRootScale" null null))
                  (`PrimitiveComponent.AddImpulse` (`/Game/BluePrint/Object/Spawn/BP_Block_Debris0.PaperSprite` _returnvalue_4) (-32.0 0.0 64.0) "None" false))
                (:`then_4`
                  (`self.SoundEffect` :!via `BlockBreak`
                    (:`BlockBreakOut`
                      (`SceneComponent.SetVisibility` (`self.PaperSprite`) false false)
                      (bind (_direction_3 _alpha_3) (`Timeline|タイムライン_0`)
                        (:`Update`
                          (`SceneComponent.K2_SetRelativeLocation` (`self.Box_Collision`) (`KismetMathLibrary.VLerp` (0.0 0.0 0.0) (0.0 0.0 4.0) _alpha_3) false false))
                        (:`Finished`
                          (`self.K2_DestroyActor`))))))))
            (:`0`
              (goto _label_2))
            (:`1`
              ;[0 0 1] UnderStyle
              (`|ExecutionSequence`
                (:`then_0`
                  (bind _returnvalue_5 (`|SpawnActorFromClass` "/Game/BluePrint/Object/Spawn/BP_Block_Debris1.BP_Block_Debris1_C" (`KismetMathLibrary.MakeTransform` (+ (4.0 0.0 4.0) (`self.K2_GetActorLocation`))) "Undefined" "OverrideRootScale" null null))
                  (`PrimitiveComponent.AddImpulse` (`/Game/BluePrint/Object/Spawn/BP_Block_Debris1.PaperSprite` _returnvalue_5) (32.0 0.0 128.0) "None" false))
                (:`then_1`
                  (bind _returnvalue_6 (`|SpawnActorFromClass` "/Game/BluePrint/Object/Spawn/BP_Block_Debris1.BP_Block_Debris1_C" (`KismetMathLibrary.MakeTransform` (+ (4.0 0.0 -4.0) (`self.K2_GetActorLocation`))) "Undefined" "OverrideRootScale" null null))
                  (`PrimitiveComponent.AddImpulse` (`/Game/BluePrint/Object/Spawn/BP_Block_Debris1.PaperSprite` _returnvalue_6) (32.0 0.0 64.0) "None" false))
                (:`then_2`
                  (bind _returnvalue_7 (`|SpawnActorFromClass` "/Game/BluePrint/Object/Spawn/BP_Block_Debris1.BP_Block_Debris1_C" (`KismetMathLibrary.MakeTransform` (+ (-4.0 0.0 4.0) (`self.K2_GetActorLocation`))) "Undefined" "OverrideRootScale" null null))
                  (`PrimitiveComponent.AddImpulse` (`/Game/BluePrint/Object/Spawn/BP_Block_Debris1.PaperSprite` _returnvalue_7) (-32.0 0.0 128.0) "None" false))
                (:`then_3`
                  (bind _returnvalue_8 (`|SpawnActorFromClass` "/Game/BluePrint/Object/Spawn/BP_Block_Debris1.BP_Block_Debris1_C" (`KismetMathLibrary.MakeTransform` (+ (-4.0 0.0 -4.0) (`self.K2_GetActorLocation`))) "Undefined" "OverrideRootScale" null null))
                  (`PrimitiveComponent.AddImpulse` (`/Game/BluePrint/Object/Spawn/BP_Block_Debris1.PaperSprite` _returnvalue_8) (-32.0 0.0 64.0) "None" false))
                (:`then_4`
                  (`self.SoundEffect` :!via `BlockBreak`
                    (:`BlockBreakOut`
                      (`SceneComponent.SetVisibility` (`self.PaperSprite`) false false)
                      (bind (_direction_4 _alpha_4) (`Timeline|タイムライン_1`)
                        (:`Update`
                          (`SceneComponent.K2_SetRelativeLocation` (`self.Box_Collision`) (`KismetMathLibrary.VLerp` (0.0 0.0 0.0) (0.0 0.0 4.0) _alpha_4) false false))
                        (:`Finished`
                          (`self.K2_DestroyActor`))))))))))))
    (:`NewEnumerator2`
      (goto _label))))

(event `self.Box_Top.OnComponentBeginOverlap`
  (params (OverlappedComponent :type "PrimitiveComponent Object Reference") (OtherActor :type "Actor Object Reference") (OtherComp :type "PrimitiveComponent Object Reference") (OtherBodyIndex :type Integer) (bFromSweep :type Boolean) (SweepResult :type "HitResult Structure (by ref)"))
  (`self.Launch` OtherActor
    (:`CastFailed`
      (`GameplayStatics.ApplyDamage` OtherActor 1.0))))

(event `self.ReceiveAnyDamage`
  (params (Damage :type "Float (single-precision)") (DamageType :type "DamageType Object Reference") (InstigatedBy :type "Controller Object Reference") (DamageCauser :type "Actor Object Reference"))
  (goto _label))

(fn `UserConstructionScript`
  (bind _papersprite (`self.PaperSprite`))
  (switch `int` (`self.Style`)
    (:`Default`
      (`PaperSpriteComponent.SetSprite` _papersprite "/Game/Art/Sprite/10_tile/10_tile_2.10_tile_2" :!label _label))
    (:`0`
      (goto _label))
    (:`1`
      (`PaperSpriteComponent.SetSprite` _papersprite "/Game/Art/Sprite/10_tile/10_tile_10.10_tile_10"))))