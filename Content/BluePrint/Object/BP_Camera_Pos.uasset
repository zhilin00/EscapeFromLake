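; BP_Camera_Pos is a placed camera actor that becomes the player's view target when the level starts with BP_Player inside its Box.
; After a brief BeginPlay delay, it tests that overlap and switches the view to itself.
; Construction shows the move trigger only when CameraMove is set.
; All overlap events are empty, leaving the blended enter/exit switching, warp delay and timeline camera slide disconnected.
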(event `self.ReceiveBeginPlay`
  (`KismetSystemLibrary.Delay` 0.01)
  (bind _asbp_player (cast `/Game/BluePrint/BP_Player` (`GameplayStatics.GetPlayerPawn` 0)))
  (if (`PrimitiveComponent.IsOverlappingActor` (`self.Box`) _asbp_player)
    (`PlayerController.SetViewTargetWithBlend` (`GameplayStatics.GetPlayerController` 0) self 0.0 "VTBlend_Linear" 0.0 false)))

(event `self.Box.OnComponentBeginOverlap`
  (params (OverlappedComponent :type "PrimitiveComponent Object Reference") (OtherActor :type "Actor Object Reference") (OtherComp :type "PrimitiveComponent Object Reference") (OtherBodyIndex :type Integer) (bFromSweep :type Boolean) (SweepResult :type "HitResult Structure (by ref)")))

(event `self.Box.OnComponentEndOverlap`
  (params (OverlappedComponent :type "PrimitiveComponent Object Reference") (OtherActor :type "Actor Object Reference") (OtherComp :type "PrimitiveComponent Object Reference") (OtherBodyIndex :type Integer)))

(event `self.Box_Move_Trigger.OnComponentBeginOverlap`
  (params (OverlappedComponent :type "PrimitiveComponent Object Reference") (OtherActor :type "Actor Object Reference") (OtherComp :type "PrimitiveComponent Object Reference") (OtherBodyIndex :type Integer) (bFromSweep :type Boolean) (SweepResult :type "HitResult Structure (by ref)")))

(fn `UserConstructionScript`
  (bind _box_move_trigger (`self.Box_Move_Trigger`))
  (if (`self.Camera_Move`)
    (`SceneComponent.SetVisibility` _box_move_trigger true false)
    (else
      (`SceneComponent.SetVisibility` _box_move_trigger false false))))