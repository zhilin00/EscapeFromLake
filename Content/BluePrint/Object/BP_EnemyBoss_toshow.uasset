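; Necromancer boss enemy for a 2D flipbook game that paces forward, reversing when a hit stops it.
; A looping timer started from Tick randomly summons a skull, flame cylinder or explosion at random positions, each followed by SkillBullet's seven-fireball spread, spawned twice.
; Four overlap boxes damage the player, or the boss during player melee.
; Damage flashes a hurt flipbook; health reaching exactly zero awards 1000 points and removes the boss.
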(event `self.ReceiveBeginPlay`
  ;[1 1 1] Begin_Rotation
  (`self.K2_SetActorRotation` (`KismetMathLibrary.ComposeRotators` (struct :`Yaw` 180.0) (`self.K2_GetActorRotation`))))

(event `self.ReceiveTick`
  (params (DeltaSeconds :type "Float (single-precision)"))
  ;[1 1 1] Tick_Walk&Skill
  (if (`KismetSystemLibrary.K2_TimerExistsHandle` (`self.skillHandle`))
    (set `CharacterMovementComponent.MaxWalkSpeed` 30.0 (`self.CharacterMovement`))
    (`self.AddMovementInput` (`self.GetActorForwardVector`))
    (else
      (bind _returnvalue (`KismetSystemLibrary.K2_SetTimerDelegate` (delegate `BossSkill`) 2.0 true 1.0))
      (set `self.skillHandle` _returnvalue))))

(event `BossSkill`
  ;[1 1 1] Tick_Walk&Skill
  (switch `int` (`KismetMathLibrary.RandomInteger` 3)
    (:`0`
      (`/Engine/EditorBlueprintResources/StandardMacros.DoOnce` false :!label _label
        (:`Completed`
          (`PaperFlipbookComponent.SetFlipbook` (`self.Sprite`) "/Game/Art/Sprite/Necromancer_creativekind-boss_6/boss_attack3.boss_attack3")
          (bind _returnvalue (`|SpawnActorFromClass` "/Game/BluePrint/Object/BP_EnemySkull.BP_EnemySkull_C" (`KismetMathLibrary.MakeTransform` (`KismetMathLibrary.MakeVector` (`KismetMathLibrary.RandomFloatInRange` 1673.0 1941.0) 0.0 (`KismetMathLibrary.RandomFloatInRange` 24.0 182.0))) "AdjustIfPossibleButDontSpawnIfColliding" "OverrideRootScale" null null))
          (`self.SpawnDefaultController` _returnvalue)
          (`self.SkillBullet`)
          (`KismetSystemLibrary.Delay` 2.0)
          (`PaperFlipbookComponent.SetFlipbook` (`self.Sprite`) "/Game/Art/Sprite/Necromancer_creativekind-boss_6/Necromancer_creativekind_boss_move.Necromancer_creativekind_boss_move")
          (goto _label :!via `Reset`))))
    (:`1`
      (`/Engine/EditorBlueprintResources/StandardMacros.DoOnce` false :!label _label_2
        (:`Completed`
          (`PaperFlipbookComponent.SetFlipbook` (`self.Sprite`) "/Game/Art/Sprite/Necromancer_creativekind-boss_6/boss_attack2.boss_attack2")
          (bind _returnvalue_2 (`|SpawnActorFromClass` "/Game/BluePrint/Object/BP_FlameCylinder.BP_FlameCylinder_C" (`KismetMathLibrary.MakeTransform` (`KismetMathLibrary.MakeVector` (`KismetMathLibrary.RandomFloatInRange` 1673.0 1941.0) 0.0 (`KismetMathLibrary.RandomFloatInRange` 24.0 182.0))) "AlwaysSpawn" "OverrideRootScale" null null))
          (`self.SpawnDefaultController` _returnvalue_2)
          (`self.SkillBullet`)
          (`KismetSystemLibrary.Delay` 2.0)
          (`PaperFlipbookComponent.SetFlipbook` (`self.Sprite`) "/Game/Art/Sprite/Necromancer_creativekind-boss_6/Necromancer_creativekind_boss_move.Necromancer_creativekind_boss_move")
          (goto _label_2 :!via `Reset`))))
    (:`2`
      (`/Engine/EditorBlueprintResources/StandardMacros.DoOnce` false :!label _label_3
        (:`Completed`
          (`PaperFlipbookComponent.SetFlipbook` (`self.Sprite`) "/Game/Art/Sprite/Necromancer_creativekind-boss_6/boss_attack1.boss_attack1")
          (`|SpawnActorFromClass` "/Game/BluePrint/Object/BP_Explosion.BP_Explosion_C" (`KismetMathLibrary.MakeTransform` (`KismetMathLibrary.MakeVector` (`KismetMathLibrary.RandomFloatInRange` 1673.0 1941.0) 0.0 (`KismetMathLibrary.RandomFloatInRange` 24.0 182.0))) "AlwaysSpawn" "OverrideRootScale" null null)
          (`self.SpawnDefaultController`)
          (`self.SkillBullet`)
          (`KismetSystemLibrary.Delay` 2.0)
          (`PaperFlipbookComponent.SetFlipbook` (`self.Sprite`) "/Game/Art/Sprite/Necromancer_creativekind-boss_6/Necromancer_creativekind_boss_move.Necromancer_creativekind_boss_move")
          (goto _label_3 :!via `Reset`))))))

(event `self.ReceiveHit`
  (params (MyComp :type "PrimitiveComponent Object Reference") (Other :type "Actor Object Reference") (OtherComp :type "PrimitiveComponent Object Reference") (bSelfMoved :type Boolean) (HitLocation :type "Vector Structure") (HitNormal :type "Vector Structure") (NormalImpulse :type "Vector Structure") (Hit :type "HitResult Structure (by ref)"))
  (bind _returnvalue_x (`KismetMathLibrary.BreakVector` (`self.GetVelocity`)))
  ;[1 1 1] Attack&Reverse
  (if (== 0.0 _returnvalue_x)
    (`/Engine/EditorBlueprintResources/StandardMacros.DoOnce` false :!label _label_4
      (:`Completed`
        (`self.Reverse`)
        (`KismetSystemLibrary.Delay` 0.2)
        (goto _label_4 :!via `Reset`)))))

(event `self.Box_Forward.OnComponentBeginOverlap`
  (params (OverlappedComponent :type "PrimitiveComponent Object Reference") (OtherActor :type "Actor Object Reference") (OtherComp :type "PrimitiveComponent Object Reference") (OtherBodyIndex :type Integer) (bFromSweep :type Boolean) (SweepResult :type "HitResult Structure (by ref)"))
  ;[1 1 1] Attack&Reverse
  (bind _asbp_player (cast `/Game/BluePrint/BP_Player` OtherActor))
  (if (`/Game/BluePrint/BP_Player.bMelee_Attack` _asbp_player)
    (`GameplayStatics.ApplyDamage` self 1.0)
    (else
      (`GameplayStatics.ApplyDamage` _asbp_player 1.0))))

(event `self.Box_Back.OnComponentBeginOverlap`
  (params (OverlappedComponent :type "PrimitiveComponent Object Reference") (OtherActor :type "Actor Object Reference") (OtherComp :type "PrimitiveComponent Object Reference") (OtherBodyIndex :type Integer) (bFromSweep :type Boolean) (SweepResult :type "HitResult Structure (by ref)"))
  ;[1 1 1] Attack&Reverse
  (bind _asbp_player (cast `/Game/BluePrint/BP_Player` OtherActor))
  (if (`/Game/BluePrint/BP_Player.bMelee_Attack` _asbp_player)
    (`GameplayStatics.ApplyDamage` self 1.0)
    (else
      (`GameplayStatics.ApplyDamage` _asbp_player 1.0))))

(event `self.Box_Top_Forward.OnComponentBeginOverlap`
  (params (OverlappedComponent :type "PrimitiveComponent Object Reference") (OtherActor :type "Actor Object Reference") (OtherComp :type "PrimitiveComponent Object Reference") (OtherBodyIndex :type Integer) (bFromSweep :type Boolean) (SweepResult :type "HitResult Structure (by ref)"))
  ;[1 1 1] Attack&Reverse
  (bind _asbp_player (cast `/Game/BluePrint/BP_Player` OtherActor))
  (if (`/Game/BluePrint/BP_Player.bMelee_Attack` _asbp_player)
    (`GameplayStatics.ApplyDamage` self 1.0)
    (else
      (`GameplayStatics.ApplyDamage` _asbp_player 1.0))))

(event `self.Box_Top_Back.OnComponentBeginOverlap`
  (params (OverlappedComponent :type "PrimitiveComponent Object Reference") (OtherActor :type "Actor Object Reference") (OtherComp :type "PrimitiveComponent Object Reference") (OtherBodyIndex :type Integer) (bFromSweep :type Boolean) (SweepResult :type "HitResult Structure (by ref)"))
  ;[1 1 1] Attack&Reverse
  (bind _asbp_player (cast `/Game/BluePrint/BP_Player` OtherActor))
  (if (`/Game/BluePrint/BP_Player.bMelee_Attack` _asbp_player)
    (`GameplayStatics.ApplyDamage` self 1.0)
    (else
      (`GameplayStatics.ApplyDamage` _asbp_player 1.0))))

(event `self.ReceiveAnyDamage`
  (params (Damage :type "Float (single-precision)") (DamageType :type "DamageType Object Reference") (InstigatedBy :type "Controller Object Reference") (DamageCauser :type "Actor Object Reference"))
  (bind _returnvalue (- (`self.iHealth`) Damage))
  ;[1 1 1] Hit_Death
  (if (== _returnvalue 0.0)
    (`/Game/BluePrint/BP_GameInstance.Get_Point` (cast `/Game/BluePrint/BP_GameInstance` (`GameplayStatics.GetGameInstance`) :!pure true) 1000)
    (`PaperFlipbookComponent.SetFlipbook` (`self.Sprite`) "/Game/Art/Sprite/Necromancer_creativekind-boss_6/boss_death.boss_death")
    (`GameplayStatics.PlaySound2D` "/Game/Sound/SE/SE_Stomp.SE_Stomp" 1.0 1.0 0.0 null null)
    (`|SpawnActorFromClass` "/Game/BluePrint/Object/Spawn/BP_Text_1000.BP_Text_1000_C" (`KismetMathLibrary.MakeTransform` (+ (0.0 0.0 16.0) (`self.K2_GetActorLocation`))) "Undefined" "OverrideRootScale" null null)
    (`CharacterMovementComponent.DisableMovement` (`self.CharacterMovement`))
    (`self.SetActorEnableCollision` false)
    (`self.SetLifeSpan` 1.0)
    (else
      (set `self.iHealth` _returnvalue)
      (`/Engine/EditorBlueprintResources/StandardMacros.DoOnce` false :!label _label_5
        (:`Completed`
          (`PaperFlipbookComponent.SetFlipbook` (`self.Sprite`) "/Game/Art/Sprite/Necromancer_creativekind-boss_6/Necromancer_creativekind_boss_damage.Necromancer_creativekind_boss_damage")
          (`KismetSystemLibrary.Delay` 0.3)
          (`PaperFlipbookComponent.SetFlipbook` (`self.Sprite`) "/Game/Art/Sprite/Necromancer_creativekind-boss_6/Necromancer_creativekind_boss_move.Necromancer_creativekind_boss_move")
          (goto _label_5 :!via `Reset`))))))

(fn `Reverse`
  (`self.K2_SetActorRotation` (`KismetMathLibrary.ComposeRotators` (struct :`Yaw` 180.0) (`self.K2_GetActorRotation`))))

(fn `SkillBullet`
  (bind _returnvalue_x (`KismetMathLibrary.BreakVector` (`self.GetActorForwardVector`)))
  (bind _returnvalue_x_2 (`KismetMathLibrary.BreakVector` (`self.GetActorForwardVector`)))
  (bind _returnvalue_x_3 (`KismetMathLibrary.BreakVector` (`self.GetActorForwardVector`)))
  (bind _returnvalue_x_4 (`KismetMathLibrary.BreakVector` (`self.GetActorForwardVector`)))
  (bind _returnvalue_x_5 (`KismetMathLibrary.BreakVector` (`self.GetActorForwardVector`)))
  (bind _returnvalue_x_6 (`KismetMathLibrary.BreakVector` (`self.GetActorForwardVector`)))
  (`|ExecutionSequence`
    (:`then_0`
      _)
    (:`then_1`
      _))
  (bind _returnvalue (`|SpawnActorFromClass` "/Game/BluePrint/Object/BP_Fireball_Boss.BP_Fireball_Boss_C" (`SceneComponent.K2_GetComponentToWorld` (`self.Fire_Ball_Pos1`)) "AlwaysSpawn" "OverrideRootScale" null null))
  (`self.SpawnDefaultController` _returnvalue)
  (`self.K2_SetActorRotation` _returnvalue (struct :`Pitch` 180.0) false)
  (`self.LaunchCharacter` _returnvalue (`KismetMathLibrary.MakeVector` (* -200.0 _returnvalue_x_3)) false false)
  (bind _returnvalue_2 (`|SpawnActorFromClass` "/Game/BluePrint/Object/BP_Fireball_Boss.BP_Fireball_Boss_C" (`SceneComponent.K2_GetComponentToWorld` (`self.Fire_Ball_Pos2`)) "AlwaysSpawn" "OverrideRootScale" null null))
  (`self.SpawnDefaultController` _returnvalue_2)
  (`self.K2_SetActorRotation` _returnvalue_2 (struct :`Pitch` 150.0) false)
  (`self.LaunchCharacter` _returnvalue_2 (`KismetMathLibrary.MakeVector` (* -173.0 _returnvalue_x_4) 0.0 100.0) false false)
  (bind _returnvalue_3 (`|SpawnActorFromClass` "/Game/BluePrint/Object/BP_Fireball_Boss.BP_Fireball_Boss_C" (`SceneComponent.K2_GetComponentToWorld` (`self.Fire_Ball_Pos3`)) "AlwaysSpawn" "OverrideRootScale" null null))
  (`self.SpawnDefaultController` _returnvalue_3)
  (`self.K2_SetActorRotation` _returnvalue_3 (struct :`Pitch` 120.0) false)
  (`self.LaunchCharacter` _returnvalue_3 (`KismetMathLibrary.MakeVector` (* -100.0 _returnvalue_x_5) 0.0 173.0) false false)
  (bind _returnvalue_4 (`|SpawnActorFromClass` "/Game/BluePrint/Object/BP_Fireball_Boss.BP_Fireball_Boss_C" (`SceneComponent.K2_GetComponentToWorld` (`self.Fire_Ball_Pos4`)) "AlwaysSpawn" "OverrideRootScale" null null))
  (`self.SpawnDefaultController` _returnvalue_4)
  (`self.K2_SetActorRotation` _returnvalue_4 (struct :`Pitch` 90.0) false)
  (`self.LaunchCharacter` _returnvalue_4 (0.0 0.0 200.0) false false)
  (bind _returnvalue_5 (`|SpawnActorFromClass` "/Game/BluePrint/Object/BP_Fireball_Boss.BP_Fireball_Boss_C" (`SceneComponent.K2_GetComponentToWorld` (`self.Fire_Ball_Pos5`)) "AlwaysSpawn" "OverrideRootScale" null null))
  (`self.SpawnDefaultController` _returnvalue_5)
  (`self.K2_SetActorRotation` _returnvalue_5 (struct :`Pitch` 60.0) false)
  (`self.LaunchCharacter` _returnvalue_5 (`KismetMathLibrary.MakeVector` (* 100.0 _returnvalue_x_6) 0.0 173.0) false false)
  (bind _returnvalue_6 (`|SpawnActorFromClass` "/Game/BluePrint/Object/BP_Fireball_Boss.BP_Fireball_Boss_C" (`SceneComponent.K2_GetComponentToWorld` (`self.Fire_Ball_Pos6`)) "AlwaysSpawn" "OverrideRootScale" null null))
  (`self.SpawnDefaultController` _returnvalue_6)
  (`self.K2_SetActorRotation` _returnvalue_6 (struct :`Pitch` 30.0) false)
  (`self.LaunchCharacter` _returnvalue_6 (`KismetMathLibrary.MakeVector` (* 173.0 _returnvalue_x) 0.0 100.0) false false)
  (bind _returnvalue_7 (`|SpawnActorFromClass` "/Game/BluePrint/Object/BP_Fireball_Boss.BP_Fireball_Boss_C" (`SceneComponent.K2_GetComponentToWorld` (`self.Fire_Ball_Pos7`)) "AlwaysSpawn" "OverrideRootScale" null null))
  (`self.SpawnDefaultController` _returnvalue_7)
  (`self.LaunchCharacter` _returnvalue_7 (`KismetMathLibrary.MakeVector` (* -200.0 _returnvalue_x_2)) false false))

(fn `UserConstructionScript`)