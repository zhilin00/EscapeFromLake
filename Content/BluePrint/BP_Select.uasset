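; BP_Select is a level-routing Blueprint that opens the 00Start level as soon as it begins play.
; Number keys jump between start, test and gameplay levels, R and C run restart and show-collision console commands, and input actions toggle pause with a sound or quit.
; An unconnected chain would show a select HUD, wait, then switch levels, including game over, on the game instance's Level value.
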(event `self.ReceiveBeginPlay`
  (`GameplayStatics.OpenLevel` "00Start"))

(event `Key|Zero`
  (params (Key :type "Key Structure"))
  ;[1 1 1] Command
  (:`Pressed`
    (`GameplayStatics.OpenLevel` "10Test")))

(event `InputAction|Pause` :paused true
  (params (Key :type "Key Structure"))
  ;[1 1 1] Command
  (:`Pressed`
    (if (`GameplayStatics.IsGamePaused`)
      (`GameplayStatics.SetGamePaused` false)
      (else
        (`GameplayStatics.SetGamePaused` true)))
    (`GameplayStatics.PlaySound2D` "/Game/Sound/SE/SE_Pause.SE_Pause" 1.0 1.0 0.0 null null)))

(event `Key|One`
  (params (Key :type "Key Structure"))
  ;[1 1 1] Command
  (:`Pressed`
    (`GameplayStatics.OpenLevel` "00Start")))

(event `Key|R`
  (params (Key :type "Key Structure"))
  ;[1 1 1] Command
  (:`Pressed`
    (`KismetSystemLibrary.ExecuteConsoleCommand` "ReStartLevel" null)))

(event `Key|Two`
  (params (Key :type "Key Structure"))
  ;[1 1 1] Command
  (:`Pressed`
    (`GameplayStatics.OpenLevel` "11Level")))

(event `Key|Three`
  (params (Key :type "Key Structure"))
  ;[1 1 1] Command
  (:`Pressed`
    (`GameplayStatics.OpenLevel` "12Level")))

(event `InputAction|Quit` :paused true
  (params (Key :type "Key Structure"))
  ;[1 1 1] Command
  (:`Pressed`
    (`KismetSystemLibrary.QuitGame` null "Quit")))

(event `Key|C`
  (params (Key :type "Key Structure"))
  ;[1 1 1] Command
  (:`Pressed`
    (`KismetSystemLibrary.ExecuteConsoleCommand` "Show Collision" null)))

(fn `UserConstructionScript`)