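; BP_Start drives the game's start screen, resetting the run and starting play on any key press.
; BeginPlay sets a windowed resolution, shows the cursor, resets score, coins, lives, level, restart position and power-up in BP_GameInstance, then displays the BP_Start_HUD widget.
; Any key sets level 2 and opens 10Test.
; Other inputs toggle pause with sound, quit, or serve as debug shortcuts for level jumps, restarting and collision display.
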(event `self.ReceiveBeginPlay`
  (`KismetSystemLibrary.ExecuteConsoleCommand` "r.SetRes 1280x720w" null)
  (set `PlayerController.bShowMouseCursor` true (`GameplayStatics.GetPlayerController` 0))
  (bind _asbp_game_instance (cast `/Game/BluePrint/BP_GameInstance` (`GameplayStatics.GetGameInstance`)))
  (set `/Game/BluePrint/BP_GameInstance.PointCount` 0 _asbp_game_instance)
  (set `/Game/BluePrint/BP_GameInstance.CoinCount` 0 _asbp_game_instance)
  (set `/Game/BluePrint/BP_GameInstance.LifeCount` 3 _asbp_game_instance)
  (set `/Game/BluePrint/BP_GameInstance.Level` 1 _asbp_game_instance)
  (`/Game/BluePrint/BP_GameInstance.LevelText` _asbp_game_instance)
  (set `/Game/BluePrint/BP_GameInstance.ReStartPos` (0.0 0.0 0.0) _asbp_game_instance)
  (set `/Game/BluePrint/BP_GameInstance.PowerUp` "NewEnumerator0" _asbp_game_instance)
  (bind _returnvalue (`|CreateWidget` "/Game/BluePrint/HUD/BP_Start_HUD.BP_Start_HUD_C"))
  (`UserWidget.AddToViewport` _returnvalue 0))

(event `Key|AnyKey`
  (params (Key :type "Key Structure"))
  (:`Pressed`
    (bind _asbp_game_instance (cast `/Game/BluePrint/BP_GameInstance` (`GameplayStatics.GetGameInstance`)))
    (set `/Game/BluePrint/BP_GameInstance.Level` 2 _asbp_game_instance)
    (`/Game/BluePrint/BP_GameInstance.LevelText` _asbp_game_instance)
    (`GameplayStatics.OpenLevel` "10Test")))

(event `Key|Zero`
  (params (Key :type "Key Structure"))
  ;[1 1 1] Command
  (:`Pressed`
    (`GameplayStatics.OpenLevel` "10Test")))

(event `InputAction|Pause` :paused true
  (params (Key :type "Key Structure"))
  ;[1 1 1] Command
  (:`Pressed`
    (if (`GameplayStatics.IsGamePaused`)
      (`GameplayStatics.SetGamePaused` false)
      (else
        (`GameplayStatics.SetGamePaused` true)))
    (`GameplayStatics.PlaySound2D` "/Game/Sound/SE/SE_Pause.SE_Pause" 1.0 1.0 0.0 null null)))

(event `Key|One`
  (params (Key :type "Key Structure"))
  ;[1 1 1] Command
  (:`Pressed`
    (`GameplayStatics.OpenLevel` "00Start")))

(event `Key|R`
  (params (Key :type "Key Structure"))
  ;[1 1 1] Command
  (:`Pressed`
    (`KismetSystemLibrary.ExecuteConsoleCommand` "ReStartLevel" null)))

(event `Key|Two`
  (params (Key :type "Key Structure"))
  ;[1 1 1] Command
  (:`Pressed`
    (`GameplayStatics.OpenLevel` "11Level")))

(event `Key|Three`
  (params (Key :type "Key Structure"))
  ;[1 1 1] Command
  (:`Pressed`
    (`GameplayStatics.OpenLevel` "12Level")))

(event `InputAction|Quit` :paused true
  (params (Key :type "Key Structure"))
  ;[1 1 1] Command
  (:`Pressed`
    (`KismetSystemLibrary.QuitGame` null "Quit")))

(event `Key|C`
  (params (Key :type "Key Structure"))
  ;[1 1 1] Command
  (:`Pressed`
    (`KismetSystemLibrary.ExecuteConsoleCommand` "Show Collision" null)))

(fn `UserConstructionScript`)